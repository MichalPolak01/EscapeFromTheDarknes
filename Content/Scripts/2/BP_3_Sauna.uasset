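; BP_3_Sauna is a door actor, apparently for a sauna, that swings open and closed and signals when the player lacks Key3.
; OpenDoor alternates through a FlipFlop between playing and reversing a timeline that lerps the door's yaw, with no key check of its own.
; A Box overlap shows the UI_Close_Door widget to a first-person character without Key3.
; Ending any overlap removes all widgets.
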(event `Open Door`
  (`/Engine/EditorBlueprintResources/StandardMacros.FlipFlop`
    (:`A`
      (bind (_direction _doorfloat) (`Timeline|Oś czasu` :!via `PlayFromStart` :!label _label)
        (:`Update`
          (`SceneComponent.K2_SetRelativeRotation` (`self.Door`) (`KismetMathLibrary.MakeRotator` 0.0 0.0 (`KismetMathLibrary.Lerp` 0.0 -100.0 _doorfloat)) false false))))
    (:`B`
      (goto _label :!via `Reverse`))))

(event `self.Box.OnComponentBeginOverlap`
  (params (OverlappedComponent :type "PrimitiveComponent Object Reference") (OtherActor :type "Actor Object Reference") (OtherComp :type "PrimitiveComponent Object Reference") (OtherBodyIndex :type Integer) (bFromSweep :type Boolean) (SweepResult :type "HitResult Structure (by ref)"))
  (bind _asbp_first_person_character (cast `/Game/FirstPerson/Blueprints/BP_FirstPersonCharacter` OtherActor))
  (if (not (`/Game/FirstPerson/Blueprints/BP_FirstPersonCharacter.Key_3` _asbp_first_person_character))
    (bind _returnvalue (`|CreateWidget` "/Game/Scripts/UI/UI_Close_Door.UI_Close_Door_C"))
    (`UserWidget.AddToViewport` _returnvalue 0)))

(event `self.Box.OnComponentEndOverlap`
  (params (OverlappedComponent :type "PrimitiveComponent Object Reference") (OtherActor :type "Actor Object Reference") (OtherComp :type "PrimitiveComponent Object Reference") (OtherBodyIndex :type Integer))
  (`WidgetLayoutLibrary.RemoveAllWidgets`))

(fn `UserConstructionScript`)